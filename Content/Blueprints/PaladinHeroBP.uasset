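; Player paladin character for a side-scrolling game, with left/right movement, jump, roll and a three-hit sword combo.
; State flags gate actions; montage-driven events end rolls and attacks, chain buffered combo clicks and toggle the sword capsule's collision.
; Sword overlaps apply tag-filtered point damage with camera shake.
; Incoming damage updates the HP bar, shows text, sound and red flash, and handles death; heart pickups only spawn an effect and disappear.
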(event OnComponentBeginOverlap(CapsuleComponent)
  (params (OverlappedComponent :type Primitive%20Component%20Object%20Reference) (OtherActor :type Actor%20Object%20Reference) (OtherComp :type Primitive%20Component%20Object%20Reference) (OtherBodyIndex :type Integer) (bFromSweep :type Boolean) (SweepResult :type Hit%20Result%20Structure%20%28by%20ref%29))
  (if (Utilities|Name|Equal(Name) (Utilities|Array|Get(acopy) (Variables|/Script/Engine.Actor|GetTags OtherActor)) "HeartItem")
    (Actor|DestroyActor OtherActor)
    (Effects|SpawnEmitterAttached "/Game/InfinityBladeEffects/Effects/FX_Ability/Heal/P_HealthPotion_Pickup_01.P_HealthPotion_Pickup_01" (Variables|Default|GetHpEmitterPosDummy) "None")))

(event EventBeginPlay
  (Game|Player|SetViewTargetwithBlend (Game|GetPlayerController 0) (Variables|Default|GetCam) 0.0 "VTBlend_Linear" 0.0 false)
  (bind _asside_scroll_game_instance (Utilities|Casting|CastToSideScrollGameInstance (Game|GetGameInstance)))
  (Variables|Default|SetSideScrollGameInsRef _asside_scroll_game_instance))

(fn ConstructionScript)

(fn CreateDamageText
  (params (Damage :type Float%20%28double-precision%29))
  (bind _returnvalue (Game|SpawnActorfromClass "/Game/Blueprints/Etc/CharDamageTextBP.CharDamageTextBP_C" (Math|Transform|MakeTransform (+ (Transformation|GetWorldLocation (Variables|Default|GetCube_DamageTextPosDummy)) "-60.000000, 0, 0")) "Undefined" 0 0))
  (Default|SetDamageText _returnvalue Damage))

(fn UpdateMoveKey
  (params (AxisValue :type Float%20%28double-precision%29))
  (if (< AxisValue 0.0)
    (Variables|Default|SetIsPressRightKey false)
    (elif (> AxisValue 0.0)
      (Variables|Default|SetIsPressRightKey true))))

(fn UpdateRotbyMoveKey
  (params (IsPressRightKey :type Boolean))
  (if IsPressRightKey
    (Transformation|SetActorRotation "0,90.000000, 0")
    (else
      (Transformation|SetActorRotation "0,-90.000000, 0"))))

(event Custom|OnAnimEnd_Rolling
  (Variables|상태|SetIsRolling false))

(event EventOnLanded
  (params (Hit :type Hit%20Result%20Structure%20%28by%20ref%29))
  (Animation|StopAnimMontage "/Game/Mesh/Paladin2/AnimMontage/root_sword_and_shield_jump_Montage.root_sword_and_shield_jump_Montage"))

(event Input|AxisEvents|InputAxisLeftRight
  (params (AxisValue :type Float%20%28single-precision%29))
  (CallFunction|UpdateMoveKey AxisValue)
  (if (not (Variables|상태|GetIsRolling)) ; 구르기하고 있지 않은지 체크
    (if (not (Variables|상태|GetIsAttacking)) ; 공격중이 아닌지 체크
      (Pawn|Input|AddMovementInput "0,1.000000, 0" AxisValue false) ; 공격중이 아니고\n구르기하고 있지 않으면\n이동
    )))

(event Input|KeyboardEvents|SpaceBar
  (params (Key :type Key%20Structure :default "None"))
  (:Pressed
    (if (not (AI|Components|NavMovement|IsFalling (Variables|Character|GetCharacterMovement))) ; 공중이 아닌지 체크
      (if (not (Variables|상태|GetIsRolling)) ; 구르기하고 있지 않은지 체크
        (if (not (Variables|상태|GetIsAttacking)) ; 공격중이 아닌지 체크
          (Character|Jump) ; 공중이 아니고\n공격중이 아니고\n구르기하고 있지 않으면\n점프
          (Animation|PlayAnimMontage "/Game/Mesh/Paladin2/AnimMontage/root_sword_and_shield_jump_Montage.root_sword_and_shield_jump_Montage" 1.0 "None") ; 점프 애니메이션
        ))))
  (:Released
    (Character|StopJumping)))

(event Input|KeyboardEvents|LeftShift
  (params (Key :type Key%20Structure :default "None"))
  (:Pressed
    (if (not (AI|Components|NavMovement|IsFalling (Variables|Character|GetCharacterMovement))) ; 공중이 아닌지 체크
      (if (not (Variables|상태|GetIsAttacking)) ; 공격중이 아닌지 체크
        (if (not (Variables|상태|GetIsRolling)) ; 구르기하고 있지 않은지 체크
          (Variables|상태|SetIsRolling true) ; 공중이 아니고\n공격중이 아니고\n구르기하고 있지 않으면 \n구르기 시작
          (Animation|PlayAnimMontage "/Game/Mesh/Paladin2/AnimMontage/paladin_stand_rolling_Montage.paladin_stand_rolling_Montage" 1.0 "Start") ; 구르기 애님 몽타주 플레이
          (CallFunction|UpdateRotbyMoveKey (Variables|Default|GetIsPressRightKey)))))))

(event OnComponentBeginOverlap(Capsule)
  (params (OverlappedComponent :type Primitive%20Component%20Object%20Reference) (OtherActor :type Actor%20Object%20Reference) (OtherComp :type Primitive%20Component%20Object%20Reference) (OtherBodyIndex :type Integer) (bFromSweep :type Boolean) (SweepResult :type Hit%20Result%20Structure%20%28by%20ref%29))
  (Variables|Default|SetDamagedActor OtherActor) ; 데미지 받은 액터 즉 칼에 맞은 액터
  (Variables|Default|SetDamagedComp OtherComp) ; 데미지 받은 액터의 컴포넌트
  (Variables|Default|SetHitInfo SweepResult) ; 충돌 정보 저장
  (if (!= (Variables|Default|GetDamagedActor) self) ; 데미지 받은 액터가 자기 자신이 아닌지 체크
    (if (Utilities|Name|NotEqual(Name) (Utilities|Array|Get(acopy) (Variables|Actor|GetTags)) (Utilities|Array|Get(acopy) (Variables|/Script/Engine.Actor|GetTags (Variables|Default|GetDamagedActor)))) ; 데미지 받은 액터의 태그가 자기 자신의 태그와 다른지 체크\n태그로 같은 편인지 체크하는 건데 여기선 의미 없음
      (if (or (Utilities|Name|Equal(Name) (Utilities|Array|Get(acopy) (Variables|/Script/Engine.ActorComponent|GetComponentTags (Variables|Default|GetDamagedComp))) "Character") (Utilities|Name|Equal(Name) (Utilities|Array|Get(acopy) (Variables|/Script/Engine.ActorComponent|GetComponentTags (Variables|Default|GetDamagedComp))) "ItemBox")) ; 컴포넌트 태그 가 캐릭터와 아이템 박스인지 체크\n캐릭터 안에 컴포넌트가 많기 때문에 태그로 다시 확인
        (Game|Feedback|ClientStartCameraShake (Game|GetPlayerController 0) "/Game/Blueprints/Etc/CamShake_HeroAttack.CamShake_HeroAttack_C" 0.1 "CameraLocal" "0, 0, 0") ; 카메라 진동 - CamShake_HeroAttack파일에서 진동 값을 볼 수 있습니다.
        (Game|Damage|ApplyPointDamage (Variables|Default|GetDamagedActor) (Variables|Default|GetAtk) (Transformation|GetActorLocation (Variables|Default|GetDamagedActor)) (Variables|Default|GetHitInfo) 0 self) ; 칼 캡슐에 오버랩된 액터에게 포인트 데미지를 적용합니다.
      ))))

(event Custom|DamageEffect
  (CallFunction|CreateDamageText (Variables|Default|GetDamage)) ; 데미지 텍스트 생성
  (Audio|PlaySound2D "/Game/Sounds_CouchNights/Sword_Stab05.Sword_Stab05" 1.0 1.0 0.0 0 0) ; 데미지 사운드
  (Rendering|Material|SetMaterial (Variables|Character|GetMesh) 0 "/Game/Mesh/Paladin/Paladin_MAT_Inst.Paladin_MAT_Inst") ; 캐릭터를 빨간색으로 바꾸는 머티리얼 적용 후 0.2초 후에 다시 원 상태로 바꿉니다.
  (Utilities|FlowControl|Delay 0.2)
  (Rendering|Material|SetMaterial (Variables|Character|GetMesh) 0 "/Game/Mesh/Paladin/Paladin_MAT.Paladin_MAT"))

(event Custom|OnCollStart_Attack
  (Collision|SetCollisionEnabled (Variables|Default|GetCapsule) "QueryAndPhysics"))

(event Custom|OnCollEnd_Attack
  (Collision|SetCollisionEnabled (Variables|Default|GetCapsule) "NoCollision"))

(event Custom|OnAnim_CheckNextCombo
  (if (Variables|Default|GetIsGoNextCombo) ; 공격중에 공격키를 눌렀는지 체크
    (Variables|Default|SetIsGoNextCombo false)
    (bind _output_get (Variables|Default|SetComboCount (+ (Variables|Default|GetComboCount) 1))) ; 콤보 카운트 증가
    (switch int _output_get ; 콤보 카운트에 맞는 애니메이션 플레이
      (:1
        (Animation|PlayAnimMontage "/Game/Mesh/Paladin2/AnimMontage/root_sword_and_shield_slash_2_Montage.root_sword_and_shield_slash_2_Montage" 1.0 "None") ; 두 번째 콤보 공격 애님 몽타주 플레이
      )
      (:2
        (Animation|PlayAnimMontage "/Game/Mesh/Paladin2/AnimMontage/root_sword_and_shield_slash_3_Montage.root_sword_and_shield_slash_3_Montage" 1.0 "None") ; 세 번째 콤보 공격 애님 몽타주 플레이
      ))
    (CallFunction|UpdateRotbyMoveKey (Variables|Default|GetIsPressRightKey)) ; 공격중에 방향 바꿀 수 있기 때문에 오른쪽 방향키 눌렀는지 체크
  ))

(event Custom|OnAnimEnd_Attack
  (Variables|상태|SetIsAttacking false)
  (Variables|Default|SetIsGoNextCombo false)
  (Variables|Default|SetComboCount 0))

(event Game|Damage|EventAnyDamage
  (params (Damage :type Float%20%28single-precision%29) (DamageType :type Damage%20Type%20Object%20Reference) (InstigatedBy :type Controller%20Object%20Reference) (DamageCauser :type Actor%20Object%20Reference))
  (bind _output_get (Variables|Default|SetDamage Damage)) ; 데미지를 저장합니다.
  (Variables|Default|SetHp (- (Variables|Default|GetHp) _output_get)) ; Hp에 Damage를 뺍니다.
  (Default|UpdateHeroHPBar (Variables|/Game/Blueprints/SideScrollGameInstance.SideScrollGameInstance_C|GetGamePlayMainWidgetRef (Variables|Default|GetSideScrollGameInsRef)) (Variables|Default|GetHp) (Variables|Default|GetMaxHp)) ; 메인 유아이에 플레이어 캐릭터의 바뀐 HP를 업데이트합니다.
  (CallFunction|DamageEffect)
  (if (<= (Variables|Default|GetHp) 0.0) ; HP가 0과 같거나 작은지 체크
    (Animation|PlayAnimMontage "/Game/Mesh/Paladin2/AnimMontage/root_sword_and_shield_death_Montage.root_sword_and_shield_death_Montage" 1.0 "None") ; 죽는 애니메이션
    (Variables|상태|SetIsDeath true)
    (Input|DisableInput 0) ; 죽었으니 키를 못 누르게 인풋을 비활성화 시킵니다.
  ))

(event Input|MouseEvents|LeftMouseButton
  (params (Key :type Key%20Structure :default "None"))
  (:Pressed
    (if (not (Variables|상태|GetIsRolling)) ; 구르기하고 있지 않은지 체크
      (if (Variables|상태|GetIsAttacking) ; 공격중이 아닌지 체크
        (Variables|Default|SetIsGoNextCombo true) ; 공격중일 때 공격 키 누르면 다음 콤보 공격(다음 콤보 공격이 있으면)
        (else
          (Variables|상태|SetIsAttacking true) ; 구르기하고 있지 않고\n공격중이 아니면\n공격 시작
          (Animation|PlayAnimMontage "/Game/Mesh/Paladin2/AnimMontage/root_sword_and_shield_slash_Montage.root_sword_and_shield_slash_Montage" 1.0 "None")
          (CallFunction|UpdateRotbyMoveKey (Variables|Default|GetIsPressRightKey)))))))