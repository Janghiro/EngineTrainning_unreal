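; Base goblin melee monster character that chases and attacks the Paladin player, with a floating HP bar.
; Tick gathers Y-axis-only distance and direction, driving an enum state machine that idles, follows, attacks or stands down on player death or stage clear.
; Animation events toggle the weapon capsule's tag-filtered damage overlap and choose the next action.
; Taking damage interrupts attacks, knocks it back, shows hit effects and damage text, then plays impact or death.
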(event EventBeginPlay
  (bind _returnvalue (Game|SpawnActorfromClass "/Game/Blueprints/Etc/CharHpBarBP.CharHpBarBP_C" (Math|Transform|MakeTransform (Transformation|GetWorldLocation (Variables|Default|GetCube_HpBarPosDummy))) "Undefined" 0 0)) ; Cube_HpBarPosDummy에 Hp 바 위젯을 생성해서 변수에 저장합니다.
  (Variables|Default|SetCharHpBarActor _returnvalue))

(fn ConstructionScript)

(fn CreateDamageText
  (params (Damage :type Float%20%28double-precision%29))
  (bind _returnvalue (Game|SpawnActorfromClass "/Game/Blueprints/Etc/CharDamageTextBP.CharDamageTextBP_C" (Math|Transform|MakeTransform (+ (Transformation|GetWorldLocation (Variables|Default|GetCube_DamageTextPosDummy)) "-50.000000, 0, 0")) "Undefined" 0 0))
  (Default|SetDamageText _returnvalue Damage))

(event Custom|SaveDisAndDir
  (bind _returnvalue (Game|GetPlayerCharacter 0))
  (bind _returnvalue_2 (Transformation|GetActorLocation))
  (bind _returnvalue_3 (Transformation|GetActorLocation _returnvalue))
  (bind _returnvalue_4 (- _returnvalue_3 _returnvalue_2))
  (bind _y (Math|Vector|BreakVector _returnvalue_4))
  (bind _returnvalue_5 (Math|Vector|MakeVector 0.0 _y 0.0))
  (bind _asdefault_play_game_mode (Utilities|Casting|CastToDefaultPlayGameMode (Game|GetGameMode)))
  (Variables|Default|SetIsStageClear (Utilities|Enum|Equal(Enum) (Variables|/Game/Blueprints/DefaultPlayGameMode.DefaultPlayGameMode_C|GetCurGamePlayState _asdefault_play_game_mode) "NewEnumerator2")) ; 플레이어 캐릭터가 현재 스테이지를 깼는지 체크해서 저장합니다.
  (bind _aspaladin_hero_bp (Utilities|Casting|CastToPaladinHeroBP (Game|GetPlayerCharacter 0)))
  (Variables|Default|SetIsDeathPlayerChar (Variables|/Game/Blueprints/PaladinHeroBP.PaladinHeroBP_C|GetIsDeath _aspaladin_hero_bp)) ; 플레이어 캐릭터 즉 PaladinHeroBP가 죽었는지 변수에 저장합니다.
  (Variables|Default|SetDistancePlayerChar (Math|Vector|VectorLength _returnvalue_5)) ; 플레이어 캐릭터와 거리를 계산해서 저장합니다.
  (Variables|Default|SetDirToPlayerChar (Math|Vector|Normalize _returnvalue_5)) ; 플레이어 캐릭터쪽 방향을 저장합니다.
)

(event Custom|NextActionDecision
  (Variables|상태|SetIsAttacking false) ; 공격중일 수도 있어서 체크를 해제합니다.
  (if (or (Variables|Default|GetIsDeathPlayerChar) (Variables|Default|GetIsStageClear)) ; 플레이어 캐릭터가 죽었거나 \n플레이어가 스테이지어를 클리어 했는지 체크합니다.
    (Variables|상태|SetCurState "NewEnumerator3") ; 준비 상태로 바꿉니다.
    (elif (> (Variables|Default|GetDistancePlayerChar) 1.8e+02) ; 플레이어와의 거리가 180 센티미터 보다 큰지 체크합니다.
      (Variables|상태|SetCurState "NewEnumerator1") ; 플레이어를 쫒아가는 상태로 바꿉니다.
      (else
        (Variables|상태|SetCurState "NewEnumerator2") ; 공격 상태로 바꿉니다.
        (Transformation|SetActorRotation (Math|Conversions|RotationFromXVector (Variables|Default|GetDirToPlayerChar))) ; 플레이어 캐릭터를 바라보게끔 방향으로 회전 시킵니다.
        (Animation|PlayAnimMontage "/Game/Mesh/Monster/AnimMontage/golblin_slash_Montage.golblin_slash_Montage" 1.0 "None") ; 공격 애님 몽타주를 플레이합니다.
        (Variables|상태|SetIsAttacking true) ; 공격중이라고 체크합니다. 공격 애니메이션 플레이 중이라는 의미로 사용하고 있습니다.
      ))))

(event EventTick
  (params (DeltaSeconds :type Float%20%28single-precision%29))
  (bind _charhpbaractor (Variables|Default|GetCharHpBarActor))
  (CallFunction|SaveDisandDir :!pinned true) ; 판단에 필요한 정보를 수집합니다.
  (Utilities|IsValid _charhpbaractor
    (:Is%20Valid
      (Default|UpdateLocation _charhpbaractor (Transformation|GetWorldLocation (Variables|Default|GetCube_HpBarPosDummy))) ; Hp bar 위치를 업데이트합니다.
    )
    (:Is%20Not%20Valid
      _))
  (if (or (Variables|Default|GetIsDeathPlayerChar) (Variables|Default|GetIsStageClear)) ; 플레이어 캐릭터가 죽었거나 \n플레이어가 스테이지어를 클리어 했는지 체크합니다.
    (Variables|상태|SetCurState "NewEnumerator3") ; 준비 상태로 바꿉니다.
  )
  (switch Utilities|FlowControl|Switch|SwitchonMonsterState (Variables|상태|GetCurState)
    (:NewEnumerator0
      (if (<= (Variables|Default|GetDistancePlayerChar) 5e+02) ; 전투 대기 상태일 때는 플레이어 캐릭터와 거리가 5미터 이내이면 쫒아갑니다.
        (Variables|상태|SetCurState "NewEnumerator1")))
    (:NewEnumerator1
      (if (<= (Variables|Default|GetDistancePlayerChar) 1.6e+02) ; 쫒아가는 상태일때는 플레이어와 거리가 1.6 미터보다 작으면 멈추고 공격합니다.
        (Variables|상태|SetCurState "NewEnumerator2")
        (Animation|PlayAnimMontage "/Game/Mesh/Monster/AnimMontage/golblin_slash_Montage.golblin_slash_Montage" 1.0 "None")
        (Variables|상태|SetIsAttacking true)
        (else
          (Pawn|Input|AddMovementInput (Variables|Default|GetDirToPlayerChar) 1.0 false))))
    (:NewEnumerator2
      (if (not (Variables|상태|GetIsAttacking)) ; 공격 상태일 경우 공격 애니메이션 플레이 중이 아니고 거리가 1.8 미터보다 커지면 쫒아갑니다.
        (if (> (Variables|Default|GetDistancePlayerChar) 1.8e+02)
          (Variables|상태|SetCurState "NewEnumerator1"))))))

(event OnComponentBeginOverlap(Capsule)
  (params (OverlappedComponent :type Primitive%20Component%20Object%20Reference) (OtherActor :type Actor%20Object%20Reference) (OtherComp :type Primitive%20Component%20Object%20Reference) (OtherBodyIndex :type Integer) (bFromSweep :type Boolean) (SweepResult :type Hit%20Result%20Structure%20%28by%20ref%29))
  (Variables|Default|SetTempOtherActor OtherActor)
  (Variables|Default|SetTempOtherComp OtherComp)
  (if (!= (Variables|Default|GetTempOtherActor) self) ; 칼 캡슐에 충돌 된 액터가 자기 자신이 아닌지 체크합니다.
    (if (Utilities|Name|NotEqual(Name) (Utilities|Array|Get(acopy) (Variables|Actor|GetTags)) (Utilities|Array|Get(acopy) (Variables|/Script/Engine.Actor|GetTags (Variables|Default|GetTempOtherActor)))) ; 충돌된 액터의 컴포넌트가 이 몬스터의 태그와 같지 않은지 체크합니다.\n같은 편 즉 몬스터끼리 공격 못하게 막기 위해 체크합니다.
      (if (Utilities|Name|Equal(Name) (Utilities|Array|Get(acopy) (Variables|/Script/Engine.ActorComponent|GetComponentTags (Variables|Default|GetTempOtherComp))) "Character") ; 충돌된 액터의 컴포넌트가 캐릭터인지 확인합니다. \n액터에 다른 콤포넌트도 있기 때문에 한번 더 체크합니다.
        (Game|Damage|ApplyDamage (Variables|Default|GetTempOtherActor) (Variables|Default|GetAtk) 0 self) ; 칼에 맞은 액터 즉 플레이어 캐릭터에 데미지를 적용합니다.
      ))))

(event Custom|DamageEffect
  (Effects|SpawnEmitterAttached "/Game/InfinityBladeEffects/Effects/FX_Mobile/Fire/combat/P_FireBall_Powerup.P_FireBall_Powerup" (Variables|Collision|GetCapsuleComponent) "None") ; 피격 이펙트 생성
  (CallFunction|CreateDamageText (Variables|Default|GetDamage)) ; 데미지 텍스트 생성
  (Audio|PlaySound2D "/Game/Sounds_CouchNights/Sword_Stab05.Sword_Stab05" 1.0 1.0 0.0 0 0) ; 피격 사운드 플레이
  (Rendering|Material|SetMaterial (Variables|Character|GetMesh) 0 "/Game/Mesh/Monster/phong1_Inst.phong1_Inst") ; 캐릭터 색을 빨간색으로 바꿉니다.
  (Utilities|FlowControl|Delay 0.2) ; 0.2초 후에 다시 원래 색으로 바꿉니다.
  (Rendering|Material|SetMaterial (Variables|Character|GetMesh) 0 "/Game/Mesh/Monster/phong1.phong1"))

(event Custom|OnAnimEnd_Impact
  (CallFunction|NextActionDecision) ; 맞는 애니메이션 끝나면 다음 행동을 결정합니다.
)

(event Custom|OnAnimEnd_Attack
  (CallFunction|NextActionDecision) ; 공격 애니메이션이 끝나면 다음 어떤 해동을 할지 결정합니다.
)

(event Custom|OnColEnd_Attack
  (Collision|SetCollisionEnabled (Variables|Default|GetCapsule) "NoCollision"))

(event Custom|OnColStart_Attack
  (Collision|SetCollisionEnabled (Variables|Default|GetCapsule) "QueryAndPhysics"))

(event Game|Damage|EventAnyDamage
  (params (Damage :type Float%20%28single-precision%29) (DamageType :type Damage%20Type%20Object%20Reference) (InstigatedBy :type Controller%20Object%20Reference) (DamageCauser :type Actor%20Object%20Reference))
  (Variables|Default|SetDamage Damage)
  (if (Utilities|Enum|NotEqual(Enum) (Variables|상태|GetCurState) "NewEnumerator4") ; 죽지 않았는지 체크
    (Variables|상태|SetIsAttacking false) ; 맞는 순각 공격 중일 수도 있으니 공격을 멈춥니다.
    (Collision|SetCollisionEnabled (Variables|Default|GetCapsule) "NoCollision") ; 칼에 있는 캡슐 충돌체를 비활성화 합니다.
    (Variables|Default|SetHp (- (Variables|Default|GetHp) (Variables|Default|GetDamage))) ; Hp에 Damage를 뺍니다.
    (CallFunction|DamageEffect)
    (Default|UpdateHpBar (Variables|Default|GetCharHpBarActor) (Variables|Default|GetHp) (Variables|Default|GetMaxHp)) ; 바뀐 Hp를 Hp bar에 업데이트합니다.
    (Character|LaunchCharacter (* (* (Variables|Default|GetDirToPlayerChar) -1.0) 3e+02) false false) ; 캐릭터를 바라보는 반대 방향 즉 맞은 방향 반대로 뒤로 밀리게 합니다.
    (if (<= (Variables|Default|GetHp) 0.0) ; HP 가 영보다 같거나 작은지 체크
      (Animation|PlayAnimMontage "/Game/Mesh/Monster/AnimMontage/goblin_death_Montage.goblin_death_Montage" 1.0 "None") ; 죽은 애님 몽타주 플레이
      (Variables|상태|SetCurState "NewEnumerator4") ; 죽는 상태로 바꿈
      (Actor|DestroyActor (Variables|Default|GetCharHpBarActor)) ; Ho Bar 삭제
      (Utilities|FlowControl|Delay 5.0) ; 5초 후에 이 캐릭터도 삭제
      (Actor|DestroyActor)
      (else
        (Animation|PlayAnimMontage "/Game/Mesh/Monster/AnimMontage/goblin_impact_Montage.goblin_impact_Montage" 1.0 "None") ; 맞는 애니메이션으로 플레이
        (Variables|상태|SetCurState "NewEnumerator6") ; 맞는 상태로 바꿈
      ))))