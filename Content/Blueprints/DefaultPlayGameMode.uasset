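; Game mode for side-scrolling stages that decides stage clear or mission failure.
; On BeginPlay it caches the actor tagged "Boss", then polls each tick while in the Play state.
; When the boss reaches its end state, it raises cleared-stage progress in the game instance, shows a clear widget and saves.
; If the Paladin hero dies instead, it shows MissionFailed; both outcomes show the cursor and disable player input.
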(event EventBeginPlay
  (bind _outactors (Actor|GetAllActorswithTag "Boss"))
  (bind _asboss_1monster_bp (Utilities|Casting|CastToBoss1MonsterBP (Utilities|Array|Get(acopy) _outactors)))
  (Variables|Default|SetBoss _asboss_1monster_bp))

(event EventTick
  (params (DeltaSeconds :type Float%20%28single-precision%29))
  (switch Utilities|FlowControl|Switch|SwitchonGamePlayState (Variables|Default|GetCurGamePlayState)
    (:NewEnumerator1
      (if (Utilities|Enum|Equal(Enum) (Variables|/Game/Blueprints/Boss1MonsterBP.Boss1MonsterBP_C|GetCurState (Variables|Default|GetBoss)) "NewEnumerator4")
        (Variables|Default|SetCurGamePlayState "NewEnumerator2")
        (bind _asside_scroll_game_instance (Utilities|Casting|CastToSideScrollGameInstance (Game|GetGameInstance)))
        (Variables|Default|SetGameInstRef _asside_scroll_game_instance)
        (if (> (Variables|/Game/Blueprints/SideScrollGameInstance.SideScrollGameInstance_C|GetEnterStage (Variables|Default|GetGameInstRef)) (Variables|/Game/Blueprints/SideScrollGameInstance.SideScrollGameInstance_C|GetClearStage (Variables|Default|GetGameInstRef)))
          (Variables|/Game/Blueprints/SideScrollGameInstance.SideScrollGameInstance_C|SetClearStage (Variables|Default|GetGameInstRef) (Variables|/Game/Blueprints/SideScrollGameInstance.SideScrollGameInstance_C|GetEnterStage (Variables|Default|GetGameInstRef))))
        (bind _returnvalue (UserInterface|CreateWidget "/Game/Blueprints/Widgets/StageClear.StageClear_C" (Game|GetPlayerController 0)))
        (UserInterface|Viewport|AddtoViewport _returnvalue 0)
        (Variables|/Script/Engine.PlayerController|SetbShowMouseCursor (Game|GetPlayerController 0) true)
        (Input|DisableInput (Game|GetPlayerCharacter 0) (Game|GetPlayerController 0))
        (bind _asside_scroll_game_instance_2 (Utilities|Casting|CastToSideScrollGameInstance (Game|GetGameInstance)))
        (Default|Save _asside_scroll_game_instance_2)
        (else
          (bind _aspaladin_hero_bp (Utilities|Casting|CastToPaladinHeroBP (Game|GetPlayerCharacter 0)))
          (if (Variables|/Game/Blueprints/PaladinHeroBP.PaladinHeroBP_C|GetIsDeath _aspaladin_hero_bp)
            (Variables|Default|SetCurGamePlayState "NewEnumerator3")
            (bind _returnvalue_2 (UserInterface|CreateWidget "/Game/Blueprints/Widgets/MissionFailed.MissionFailed_C" (Game|GetPlayerController 0)))
            (UserInterface|Viewport|AddtoViewport _returnvalue_2 0)
            (Variables|/Script/Engine.PlayerController|SetbShowMouseCursor (Game|GetPlayerController 0) true)
            (Input|DisableInput (Game|GetPlayerCharacter 0) (Game|GetPlayerController 0))))))))

(fn ConstructionScript)