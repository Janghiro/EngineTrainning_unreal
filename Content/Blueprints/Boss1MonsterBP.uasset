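; Side-scroller first boss (Mutant) that chases and attacks the PaladinHeroBP player and shows the boss HP UI.
; A Tick-driven state machine uses Y-axis distance to switch between idle, follow and attack, with a one-second timer loop unlocking a telegraphed skill swipe.
; Animation events toggle Sphere (punch) and Capsule (skill) hitboxes, which apply tag-filtered damage.
; Taking damage updates the HP bar, spawns effects and damage text, flashes red, and handles death.
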(event EventBeginPlay
  (bind _asside_scroll_game_instance (Utilities|Casting|CastToSideScrollGameInstance (Game|GetGameInstance)))
  (Variables|Default|SetSideScrollGameInsRef _asside_scroll_game_instance))

(fn ConstructionScript)

(fn CreateDamageText
  (params (Damage :type Float%20%28double-precision%29))
  (bind _returnvalue (Game|SpawnActorfromClass "/Game/Blueprints/Etc/CharDamageTextBP.CharDamageTextBP_C" (Math|Transform|MakeTransform (+ (Transformation|GetWorldLocation (Variables|Default|GetCube_DamageTextPosDummy)) "-60.000000, 0, 0")) "Undefined" 0 0))
  (Default|SetDamageText _returnvalue Damage))

(event Custom|SaveDisAndDir
  (bind _returnvalue (Game|GetPlayerCharacter 0))
  (bind _returnvalue_2 (Transformation|GetActorLocation))
  (bind _returnvalue_3 (Transformation|GetActorLocation _returnvalue))
  (bind _returnvalue_4 (- _returnvalue_3 _returnvalue_2))
  (bind _y (Math|Vector|BreakVector _returnvalue_4))
  (bind _returnvalue_5 (Math|Vector|MakeVector 0.0 _y 0.0))
  (bind _aspaladin_hero_bp (Utilities|Casting|CastToPaladinHeroBP _returnvalue))
  (Variables|Default|SetIsDeathPlayerChar (Variables|/Game/Blueprints/PaladinHeroBP.PaladinHeroBP_C|GetIsDeath _aspaladin_hero_bp)) ; 플레이어 캐릭터 즉 PaladinHeroBP가 죽었는지 변수에 저장합니다.
  (Variables|Default|SetDistancePlayerChar (Math|Vector|VectorLength _returnvalue_5)) ; 플레이어 캐릭터와 거리를 계산해서 저장합니다.
  (Variables|Default|SetDirToPlayerChar (Math|Vector|Normalize _returnvalue_5)) ; 플레이어 캐릭터쪽 방향을 저장합니다.
)

(event Custom|SkillTimeLoop
  (Utilities|FlowControl|Delay 1.0)
  (Variables|Default|SetSkillTime (+ (Variables|Default|GetSkillTime) 1.0))
  (CallFunction|SkillTimeLoop))

(event EventTick
  (params (DeltaSeconds :type Float%20%28single-precision%29))
  (CallFunction|SaveDisandDir) ; 판단에 필요한 정보를 수집합니다.
  (if (Variables|Default|GetIsDeathPlayerChar) ; 플레이어 캐릭터가 죽으면
    (Variables|Default|SetCurState "NewEnumerator3") ; 준비 상태로 바꿉니다.
  )
  (switch Utilities|FlowControl|Switch|SwitchonMonsterState (Variables|Default|GetCurState)
    (:NewEnumerator0
      (if (<= (Variables|Default|GetDistancePlayerChar) 5e+02) ; 전투 대기 상태일 때는 플레이어 캐릭터와 거리가 5미터 이내이면 쫒아갑니다.
        (Default|ShowBossUI (Variables|Default|GetSideScrollGameInsRef) true (Variables|Default|GetBossTexture))
        (Variables|Default|SetCurState "NewEnumerator1")
        (CallFunction|SkillTimeLoop)))
    (:NewEnumerator1
      (if (<= (Variables|Default|GetDistancePlayerChar) 1.3e+02) ; 쫒아가는 상태일때는 플레이어와 거리가 1.6 미터보다 작으면 멈추고 공격합니다.
        (CallFunction|StartAttack)
        (else
          (Pawn|Input|AddMovementInput (Variables|Default|GetDirToPlayerChar) 1.0 false))))
    (:NewEnumerator2
      (if (not (Variables|상태|GetIsAttacking)) ; 공격 상태일 경우 공격 애니메이션 플레이 중이 아니고 거리가 1.8 미터보다 커지면 쫒아갑니다.
        (if (> (Variables|Default|GetDistancePlayerChar) 1.5e+02)
          (Variables|Default|SetCurState "NewEnumerator1"))))))

(event OnComponentBeginOverlap(Sphere)
  (params (OverlappedComponent :type Primitive%20Component%20Object%20Reference) (OtherActor :type Actor%20Object%20Reference) (OtherComp :type Primitive%20Component%20Object%20Reference) (OtherBodyIndex :type Integer) (bFromSweep :type Boolean) (SweepResult :type Hit%20Result%20Structure%20%28by%20ref%29))
  (Variables|Default|SetTempOtherActor2 OtherActor)
  (Variables|Default|SetTempOtherComp2 OtherComp)
  (if (!= (Variables|Default|GetTempOtherActor2) self)
    (if (Utilities|Name|NotEqual(Name) (Utilities|Array|Get(acopy) (Variables|Actor|GetTags)) (Utilities|Array|Get(acopy) (Variables|/Script/Engine.Actor|GetTags (Variables|Default|GetTempOtherActor2))))
      (if (Utilities|Name|Equal(Name) (Utilities|Array|Get(acopy) (Variables|/Script/Engine.ActorComponent|GetComponentTags (Variables|Default|GetTempOtherComp2))) "Character")
        (Game|Damage|ApplyDamage (Variables|Default|GetTempOtherActor2) (Variables|Default|GetAtk) 0 self)))))

(event OnComponentBeginOverlap(Capsule)
  (params (OverlappedComponent :type Primitive%20Component%20Object%20Reference) (OtherActor :type Actor%20Object%20Reference) (OtherComp :type Primitive%20Component%20Object%20Reference) (OtherBodyIndex :type Integer) (bFromSweep :type Boolean) (SweepResult :type Hit%20Result%20Structure%20%28by%20ref%29))
  (Variables|Default|SetTempOtherActor OtherActor)
  (Variables|Default|SetTempOtherComp OtherComp)
  (if (!= (Variables|Default|GetTempOtherActor) self)
    (if (Utilities|Name|NotEqual(Name) (Utilities|Array|Get(acopy) (Variables|Actor|GetTags)) (Utilities|Array|Get(acopy) (Variables|/Script/Engine.Actor|GetTags (Variables|Default|GetTempOtherActor))))
      (if (Utilities|Name|Equal(Name) (Utilities|Array|Get(acopy) (Variables|/Script/Engine.ActorComponent|GetComponentTags (Variables|Default|GetTempOtherComp))) "Character")
        (Game|Damage|ApplyDamage (Variables|Default|GetTempOtherActor) (Variables|Default|GetSkill1Atk) 0 self)))))

(event Custom|DamageEffect
  (Effects|SpawnEmitterAttached "/Game/InfinityBladeEffects/Effects/FX_Mobile/Fire/combat/P_FireBall_Powerup.P_FireBall_Powerup" (Variables|Collision|GetCapsuleComponent) "None") ; 피격 이펙트 생성
  (CallFunction|CreateDamageText (Variables|Default|GetDamage)) ; 데미지 텍스트 생성
  (Audio|PlaySound2D "/Game/Sounds_CouchNights/Sword_Stab05.Sword_Stab05" 1.0 1.0 0.0 0 0) ; 피격 사운드 플레이
  (Rendering|Material|SetMaterial (Variables|Character|GetMesh) 0 "/Game/Mesh/Boss1/mutant_M_Inst.mutant_M_Inst") ; 캐릭터 색을 빨간색으로 바꿉니다.
  (Utilities|FlowControl|Delay 0.2) ; 0.2초 후에 다시 원래 색으로 바꿉니다.
  (Rendering|Material|SetMaterial (Variables|Character|GetMesh) 0 "/Game/Mesh/Boss1/mutant_M.mutant_M"))

(event Custom|OnColStart_Skill1Attack
  (Collision|SetCollisionEnabled (Variables|Default|GetCapsule) "QueryAndPhysics"))

(event Custom|OnAnimEnd_Attack
  (Rendering|Material|SetMaterial (Variables|Character|GetMesh) 0 "/Game/Mesh/Boss1/mutant_M.mutant_M")
  (Variables|상태|SetIsAttacking false)
  (if (Variables|Default|GetIsDeathPlayerChar)
    (Variables|Default|SetCurState "NewEnumerator3")
    (elif (> (Variables|Default|GetDistancePlayerChar) 1.8e+02)
      (Variables|Default|SetCurState "NewEnumerator1")
      (else
        (CallFunction|StartAttack)))))

(event Custom|OnColEnd_Skill1Attack
  (Collision|SetCollisionEnabled (Variables|Default|GetCapsule) "NoCollision"))

(event Custom|StartAttack
  (Variables|상태|SetIsAttacking true)
  (if (>= (Variables|Default|GetSkillTime) 1e+01)
    (Variables|Default|SetCurState "NewEnumerator5")
    (Transformation|SetActorRotation (Math|Conversions|RotationFromXVector (Variables|Default|GetDirToPlayerChar)))
    (Rendering|Material|SetMaterial (Variables|Character|GetMesh) 0 "/Game/Mesh/Boss1/mutant_M_Skill_Inst.mutant_M_Skill_Inst")
    (Variables|Default|SetSkillTime 0.0)
    (Animation|PlayAnimMontage "/Game/Mesh/Boss1/AnimMontage/mutant_flexing_muscles_Montage.mutant_flexing_muscles_Montage" 1.0 "Start")
    (Utilities|FlowControl|Delay 2.0)
    (if (Utilities|Enum|Equal(Enum) (Variables|Default|GetCurState) "NewEnumerator5")
      (Animation|PlayAnimMontage "/Game/Mesh/Boss1/AnimMontage/mutant_swiping_Montage.mutant_swiping_Montage" 1.0 "None"))
    (else
      (Variables|Default|SetCurState "NewEnumerator2")
      (Transformation|SetActorRotation (Math|Conversions|RotationFromXVector (Variables|Default|GetDirToPlayerChar)))
      (Animation|PlayAnimMontage "/Game/Mesh/Boss1/AnimMontage/mutant_punch_Montage.mutant_punch_Montage" 1.0 "None"))))

(event Custom|OnColEnd_Attack
  (Collision|SetCollisionEnabled (Variables|Default|GetSphere) "NoCollision"))

(event Custom|OnColStart_Attack
  (Collision|SetCollisionEnabled (Variables|Default|GetSphere) "QueryAndPhysics"))

(event Game|Damage|EventAnyDamage
  (params (Damage :type Float%20%28single-precision%29) (DamageType :type Damage%20Type%20Object%20Reference) (InstigatedBy :type Controller%20Object%20Reference) (DamageCauser :type Actor%20Object%20Reference))
  (bind _output_get (Variables|Default|SetDamage Damage))
  (Variables|Default|SetHp (- (Variables|Default|GetHp) _output_get))
  (Default|UpdateBossHPBar (Variables|/Game/Blueprints/SideScrollGameInstance.SideScrollGameInstance_C|GetGamePlayMainWidgetRef (Variables|Default|GetSideScrollGameInsRef)) (Variables|Default|GetHp) (Variables|Default|GetMaxHp))
  (CallFunction|DamageEffect)
  (if (<= (Variables|Default|GetHp) 0.0)
    (Animation|PlayAnimMontage "/Game/Mesh/Boss1/AnimMontage/mutant_dying_Montage.mutant_dying_Montage" 1.0 "None")
    (Variables|Default|SetCurState "NewEnumerator4")
    (Collision|SetCollisionEnabled (Variables|Collision|GetCapsuleComponent) "NoCollision")
    (Collision|SetCollisionEnabled (Variables|Default|GetCapsule) "NoCollision")
    (Collision|SetCollisionEnabled (Variables|Default|GetSphere) "NoCollision")
    (Utilities|FlowControl|Delay 5.0)
    (Actor|DestroyActor)))