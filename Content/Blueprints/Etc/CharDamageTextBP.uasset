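; Floating damage number actor that shows a hit's damage as world-space text and then removes itself.
; SetDamageText writes the floored damage value into the TextRender component.
; On BeginPlay, a timeline moves the text vertically from its spawn location and drives its X and Y scale from the same vector track, then destroys the actor when finished.
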(event EventBeginPlay
  (bind _textrender (Variables|Default|GetTextRender))
  (Variables|Default|SetStartPos (Transformation|GetActorLocation))
  (bind _newtrack_0 (Timeline|Timeline_0 Play)
    (:Update
      (Transformation|SetWorldLocation (Variables|Default|GetTextRender) (+ (Variables|Default|GetStartPos) (Math|Vector|MakeVector 0.0 0.0 (.X (Math|Vector|BreakVector _newtrack_0)))) false false)
      (Rendering|Components|TextRender|SetXScale _textrender (.Y (Math|Vector|BreakVector _newtrack_0)))
      (Rendering|Components|TextRender|SetYScale _textrender (.Y (Math|Vector|BreakVector _newtrack_0))))
    (:Finished
      (Actor|DestroyActor))))

(fn ConstructionScript)

(fn SetDamageText
  (params (Damage :type Float%20%28double-precision%29))
  (Rendering|Components|TextRender|SetText (Variables|Default|GetTextRender) (Utilities|Text|ToText(Integer) (Math|Float|Floor Damage))))