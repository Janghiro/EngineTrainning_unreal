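; Game instance for a side-scroller that owns the main UI widgets and stage-clear progress.
; Show functions lazily create the stage select and gameplay HUD widgets, cache them, and add or remove them from the viewport.
; ShowBossUI swaps the boss image and toggles the boss panel on the gameplay HUD, assuming that widget already exists.
; Save and Load copy ClearStage to and from a save game object in a single named slot.
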(fn ShowStageSelectWidget
  (params (IsShow :type Boolean))
  (Utilities|IsValid (Variables|Default|GetStageSelectWidget)
    (:Is%20Valid
      _)
    (:Is%20Not%20Valid
      (bind _returnvalue (UserInterface|CreateWidget "/Game/Blueprints/Widgets/StageSelect.StageSelect_C" (Game|GetPlayerController 0)))
      (Variables|Default|SetStageSelectWidget _returnvalue)))
  (if IsShow
    (UserInterface|Viewport|AddtoViewport (Variables|Default|GetStageSelectWidget) 0)
    (else
      (Widget|RemovefromParent (Variables|Default|GetStageSelectWidget)))))

(fn Save
  (Utilities|IsValid (Variables|Default|GetSideScrollSaveGameRef)
    (:Is%20Valid
      _)
    (:Is%20Not%20Valid
      (bind _returnvalue (SaveGame|CreateSaveGameObject "/Game/Blueprints/SideScrollSaveGameBP.SideScrollSaveGameBP_C"))
      (bind _output_get (Variables|Default|SetSideScrollSaveGameRef _returnvalue))))
  (Variables|/Game/Blueprints/SideScrollSaveGameBP.SideScrollSaveGameBP_C|SetClearStage _output_get (Variables|Default|GetClearStage))
  (SaveGame|SaveGametoSlot (Variables|Default|GetSideScrollSaveGameRef) "SideScroll"))

(fn Load
  (bind _returnvalue (SaveGame|LoadGamefromSlot "SideScroll"))
  (bind _asside_scroll_save_game_bp (Utilities|Casting|CastToSideScrollSaveGameBP _returnvalue))
  (bind _output_get (Variables|Default|SetSideScrollSaveGameRef _asside_scroll_save_game_bp))
  (Variables|Default|SetClearStage (Variables|/Game/Blueprints/SideScrollSaveGameBP.SideScrollSaveGameBP_C|GetClearStage _output_get)))

(fn ShowGamePlayMainWidget
  (params (IsShow :type Boolean))
  (Utilities|IsValid (Variables|Default|GetGamePlayMainWidgetRef)
    (:Is%20Valid
      _)
    (:Is%20Not%20Valid
      (bind _returnvalue (UserInterface|CreateWidget "/Game/Blueprints/Widgets/GamePlayMain.GamePlayMain_C" (Game|GetPlayerController 0)))
      (Variables|Default|SetGamePlayMainWidgetRef _returnvalue)))
  (if IsShow
    (UserInterface|Viewport|AddtoViewport (Variables|Default|GetGamePlayMainWidgetRef) 0)
    (else
      (Widget|RemovefromParent (Variables|Default|GetGamePlayMainWidgetRef)))))

(fn ShowBossUI
  (params (IsShow :type Boolean) (BossTexture :type Texture%202D%20Object%20Reference))
  (if IsShow
    (Default|ChangeBossImage (Variables|Default|GetGamePlayMainWidgetRef) BossTexture)
    (Widget|SetVisibility (Variables|/Game/Blueprints/Widgets/GamePlayMain.GamePlayMain_C|GetCanvasPanel_Boss (Variables|Default|GetGamePlayMainWidgetRef)) "Visible")
    (else
      (Widget|SetVisibility (Variables|/Game/Blueprints/Widgets/GamePlayMain.GamePlayMain_C|GetCanvasPanel_Boss (Variables|Default|GetGamePlayMainWidgetRef)) "Hidden"))))